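; BP_GrappleCable is a cable actor, named for a grapple, that handles its own look and removal.
; On BeginPlay it applies an orange dynamic instance of the Dither material to its CableComponent.
; DitherOut destroys the actor immediately, leaving the timeline that would animate the dither Percent before destruction disconnected and unused.
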(event Custom|DitherOut
  ;[1 1 1] DitherOut
  (Actor|DestroyActor) ; Dither Currently Not In Use,\nDestroys Instead
)

(event EventBeginPlay
  ;[0 0.1529 1] BeginPlay
  (bind _returnvalue (Rendering|Material|CreateDynamicMaterialInstance "/Game/Mats/Dither/Dither.Dither" "None" "None" :!class /Script/Engine.KismetMaterialLibrary)) ; Set Dither Material
  (Variables|Ref|SetDitherMatRef _returnvalue)
  (Rendering|Material|SetVectorParameterValue (Variables|Ref|GetDitherMatRef) "Col" "(R=1.000000,G=0.502887,B=0.000000,A=1.000000)" :!class /Script/Engine.MaterialInstanceDynamic)
  (Rendering|Material|SetMaterial (Variables|Default|GetCableComponent) 0 (Variables|Ref|GetDitherMatRef)))

(fn ConstructionScript)